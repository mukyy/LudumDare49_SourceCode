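; BP_NavProxy is a nav link proxy that makes agents jump across its smart link.
; When an agent reaches the link, it launches the agent, if it is a Character, toward the destination, overriding its current velocity.
; CalculateVelocity solves a ballistic arc from start, destination and a fixed flight time, using a hardcoded gravity constant rather than the world's setting.
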(event `self.ReceiveSmartLinkReached`
  (params (Agent :type "Actor Object Reference") (Destination :type "Vector Structure (by ref)"))
  (bind _velocity (`self.CalculateVelocity` Destination (`self.K2_GetActorLocation` Agent) 1.5))
  (bind _ascharacter (cast `Character` Agent))
  (`Character.LaunchCharacter` _ascharacter _velocity true true))

(fn `CalculateVelocity`
  (params (Destination :type "Vector Structure") (Start :type "Vector Structure") (Duration :type "Float (double-precision)"))
  (returns (Velocity :type "Vector Structure"))
  (bind _duration (`local.Duration`))
  (return (`KismetMathLibrary.MakeVector` (/ (- (.x Destination) (.x Start)) _duration) (/ (- (.y Destination) (.y Start)) _duration) (/ (- (.z Destination) (+ (.z Start) (* (`KismetMathLibrary.Square` Duration) -0.5 982.0))) _duration))))

(fn `UserConstructionScript`)