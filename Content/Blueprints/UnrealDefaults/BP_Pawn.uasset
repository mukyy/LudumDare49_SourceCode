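; A camera pawn that slides along the world Y axis from the MoveRight input axis, scaled by Speed.
; SetCameraPosition snaps its Y to the result of FindFirstPlayer, but the looping timer meant to call it is disconnected.
; FindFirstPlayer scans all TopDownCharacters for the furthest Y, only ever raising the stored LastPlayerLocation, so the tracked lead never moves back.
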(event `self.ReceiveBeginPlay`)

(event `SetCameraPosition`
  (bind _lastplayerlocationref (`self.FindFirstPlayer`))
  (`KismetSystemLibrary.PrintString` (`KismetStringLibrary.Conv_DoubleToString` (.y _lastplayerlocationref)))
  (`self.K2_SetActorLocation` (`KismetMathLibrary.MakeVector` (.x (`self.K2_GetActorLocation`)) (.y _lastplayerlocationref) (.z (`self.K2_GetActorLocation`)))))

(event `self.ReceiveTick`
  (params (DeltaSeconds :type "Float (single-precision)")))

(event `InputAxis|MoveRight`
  (params (AxisValue :type "Float (single-precision)"))
  (`self.K2_AddActorWorldOffset` (`KismetMathLibrary.MakeVector` 0.0 (* AxisValue (`self.Speed`)))))

(fn `FindFirstPlayer`
  (returns (LastPlayerLocationRef :type "Vector Structure"))
  (locals (LastPlayerLocation :type "Vector Structure" :default (0.0 -1.0000000200408773e+20 0.0)))
  (bind (_lastplayerlocation_x _lastplayerlocation_y) (`KismetMathLibrary.BreakVector` (`local.LastPlayerLocation`)))
  (bind _outactors (`GameplayStatics.GetAllActorsOfClass` "/Game/Blueprints/Actors/TopDownCharacter.TopDownCharacter_C"))
  (for _array_element _outactors
    (`/Engine/EditorBlueprintResources/StandardMacros.IsValid` _array_element
      (:`Is Valid`
        (bind _returnvalue (`self.K2_GetActorLocation` _array_element))
        (if (> (.y _returnvalue) _lastplayerlocation_y)
          (set `local.LastPlayerLocation` _returnvalue)))))
  (return (`local.LastPlayerLocation`)))

(fn `UserConstructionScript`)