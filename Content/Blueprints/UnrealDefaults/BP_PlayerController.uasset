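; Player controller that shows the mouse cursor and relays slow-down, jump and click input to the game.
; On BeginPlay it gathers all TopDownCharacter actors and, for each, binds events to its SlowDown and Jump dispatchers.
; Holding S broadcasts SlowDown as true, releasing sends false, and Space broadcasts Jump.
; Left click traces under the cursor on the Camera channel and calls TriggerMessage on the hit actor.
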(event `self.ReceiveBeginPlay`
  (set `self.bShowMouseCursor` true)
  (bind _outactors (`GameplayStatics.GetAllActorsOfClass` "/Game/Blueprints/Actors/TopDownCharacter.TopDownCharacter_C"))
  (bind _output_get (set `self.Characters` _outactors))
  (for _array_element _output_get
    (add `self.SlowDown` (`|CreateDelegate` _array_element :!event `SlowDown`))
    (add `self.Jump` (`|CreateDelegate` _array_element :!event `CallJump`))))

(event `Key|S`
  (params (Key :type "Key Structure"))
  (:`Pressed`
    (`self.SlowDown` true))
  (:`Released`
    (`self.SlowDown` false)))

(event `Key|SpaceBar`
  (params (Key :type "Key Structure"))
  (:`Pressed`
    (`self.Jump`)))

(event `Key|LeftMouseButton`
  (params (Key :type "Key Structure"))
  (:`Pressed`
    (message `/Game/Blueprints/Actors/BPI_Platform.Trigger` (`.HitActor` (`GameplayStatics.BreakHitResult` (`self.GetHitResultUnderCursorByChannel` "TraceTypeQuery2" false))))))

(fn `UserConstructionScript`)