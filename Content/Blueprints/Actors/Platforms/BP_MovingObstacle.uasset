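; BP_MovingObstacle is an obstacle that moves between two relative points and can be temporarily deactivated.
; The construction script feeds PointA, PointB and MoveDuration into an InterpToMovement component.
; Deactivate stops that component's tick and starts a cooldown timer of DeactivationTime, extending inherited cooldown logic.
; When the cooldown finishes, it gives warnings, restores the default control color and active state, then resumes movement after short delays.
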(event `self.ReceiveTick`
  (params (DeltaSeconds :type "Float (single-precision)"))
  (`parent.ReceiveTick` DeltaSeconds))

(event `self.Deactivate`
  (set `self.IsActive` false)
  (`self.EnterCooldown`)
  (`ActorComponent.SetComponentTickEnabled` (`self.InterpToMovement`) false))

(event `self.EnterCooldown`
  (`parent.EnterCooldown`)
  (bind _returnvalue (`KismetSystemLibrary.K2_SetTimerDelegate` (delegate `self.FinishCooldown`) (`self.DeactivationTime`)))
  (set `self.DeactivationCooldownHandle` _returnvalue))

(event `self.FinishCooldown`
  (`parent.FinishCooldown`)
  (`self.WarnAboutCooldown`)
  (`KismetSystemLibrary.Delay` 1.5)
  (set `self.IsActive` true)
  (`self.ChangeControlColor` (`self.DefaultControlColor`))
  (`self.WarnPlayer`)
  (`KismetSystemLibrary.Delay` 1.0)
  (`ActorComponent.SetComponentTickEnabled` (`self.InterpToMovement`) true))

(fn `UserConstructionScript`
  (bind _interptomovement (`self.InterpToMovement`))
  (`parent.UserConstructionScript`)
  (set `InterpToMovementComponent.ControlPoints` (`|MakeArray` (make `InterpControlPoint` (`self.PointA`)) (make `InterpControlPoint` (`self.PointB`))) _interptomovement)
  (set `InterpToMovementComponent.Duration` (`self.MoveDuration`) _interptomovement))