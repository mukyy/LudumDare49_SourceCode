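; Rotating platform obstacle that spins at a set speed and can be activated for manual rotation with the mouse.
; Tick sets the physics angular velocity around Y every frame.
; Activate calls ControlTheControl, disables physics and opens a gate, letting vertical mouse movement drive local yaw (with a debug print); Deactivate reverses this.
; The construction script applies a texture and palette color through a dynamic flat-color material.
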(event `self.ReceiveTick`
  (params (DeltaSeconds :type "Float (single-precision)"))
  (bind (_deltax _deltay) (`PlayerController.GetInputMouseDelta` (`GameplayStatics.GetPlayerController` 0)))
  (`parent.ReceiveTick` DeltaSeconds)
  (`|ExecutionSequence`
    (:`then_0`
      (`PrimitiveComponent.SetPhysicsAngularVelocityInDegrees` (`self.Obstacle`) (`KismetMathLibrary.MakeVector` 0.0 (`self.RotationSpeed`)) false "None"))
    (:`then_1`
      (`parent.ReceiveTick` 0.0)
      (`/Engine/EditorBlueprintResources/StandardMacros.Gate` true :!label _label
        (:`Exit`
          (`KismetSystemLibrary.PrintString` (`KismetStringLibrary.Conv_DoubleToString` _deltay))
          (`SceneComponent.K2_AddLocalRotation` (`self.Obstacle`) (`KismetMathLibrary.MakeRotator` 0.0 0.0 (* 20.0 _deltay)) false false))))))

(event `/Game/Blueprints/Actors/BPI_Platform.Activate`
  (set `self.IsActive` true)
  (`self.ControlTheControl` true)
  (`PrimitiveComponent.SetSimulatePhysics` (`self.Obstacle`) false)
  (goto _label :!via `Open`))

(event `/Game/Blueprints/Actors/BPI_Platform.Deactivate`
  (set `self.IsActive` false)
  (`self.ControlTheControl` false)
  (`PrimitiveComponent.SetSimulatePhysics` (`self.Obstacle`) true)
  (goto _label :!via `Close`))

(fn `UserConstructionScript`
  (`parent.UserConstructionScript`)
  (bind _returnvalue (`PrimitiveComponent.CreateDynamicMaterialInstance` (`self.Obstacle`) 0 "/Game/Materials/M_FlatColor.M_FlatColor" "None"))
  (bind _output_get (set `self.ObstacleInstance` _returnvalue))
  (`MaterialInstanceDynamic.SetTextureParameterValue` _output_get "DiffuseTexture" (`self.ObstacleTexture`))
  (`MaterialInstanceDynamic.SetVectorParameterValue` _output_get "Color" (`/Game/Blueprints/Other/BPL_Getters.GetColorPalette` (`self.ColorIndex`))))