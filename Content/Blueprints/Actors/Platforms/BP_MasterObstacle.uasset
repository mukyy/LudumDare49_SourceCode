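; BP_MasterObstacle is a base obstacle actor with a color-coded control object, hidden for Passive obstacles.
; Trigger, blocked during cooldown, calls Deactivate on Activated/Disabled types or Activate on Gets Controlled types, which StopTrigger deactivates.
; A dynamic material shows controlled, cooldown and blinking red warning states.
; On Tick, Activated/Disabled types feed deactivation and cooldown timer progress into a W_TrapData widget.
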(event `self.ReceiveBeginPlay`
  (bind _returnvalue (`PrimitiveComponent.CreateDynamicMaterialInstance` (`self.ControlObject`) 0 "/Game/Materials/M_FlatColor.M_FlatColor" "None"))
  (bind _output_get (set `self.M_Control_Instance` _returnvalue))
  (`MaterialInstanceDynamic.SetVectorParameterValue` _output_get "Color" (`self.DefaultControlColor`))
  (switch `/Game/Blueprints/Other/Enum_ObstacleType` (`self.ObstacleType`)
    (:`NewEnumerator3`
      (`SceneComponent.SetVisibility` (`self.ControlObject`) false false))))

(event `self.Trigger`
  (if (not (`KismetSystemLibrary.K2_IsTimerActiveHandle` (`self.TriggerCooldownHandle`)))
    (switch `/Game/Blueprints/Other/Enum_ObstacleType` (`self.ObstacleType`)
      (:`NewEnumerator0`
        (`self.Deactivate`))
      (:`NewEnumerator1`
        (`self.Activate`)))))

(event `self.StopTrigger`
  (if true
    (switch `/Game/Blueprints/Other/Enum_ObstacleType` (`self.ObstacleType`)
      (:`NewEnumerator1`
        (`self.Deactivate`)))))

(event `self.WarnPlayer`
  (bind (_direction _lerp) (`Timeline|Blink` :!via `PlayFromStart` :!label _label)
    (:`Update`
      (`MaterialInstanceDynamic.SetVectorParameterValue` (`self.M_Control_Instance`) "Color" (`KismetMathLibrary.LinearColorLerp` (`self.DefaultControlColor`) (struct :`R` 1.0 :`A` 1.0) _lerp)))))

(event `StopAllWarnings`
  (goto _label :!via `Stop`))

(event `self.EntranceToObstacle.OnComponentBeginOverlap`
  (params (OverlappedComponent :type "PrimitiveComponent Object Reference") (OtherActor :type "Actor Object Reference") (OtherComp :type "PrimitiveComponent Object Reference") (OtherBodyIndex :type Integer) (bFromSweep :type Boolean) (SweepResult :type "HitResult Structure (by ref)")))

(event `self.EnterCooldown`
  (`self.StopAllWarnings`)
  (`MaterialInstanceDynamic.SetVectorParameterValue` (`self.M_Control_Instance`) "Color" (`self.CooldownColor`))
  (bind _returnvalue (`KismetSystemLibrary.K2_SetTimerDelegate` (delegate `TriggerCooldownFinished`) (`self.TriggerCooldown`)))
  (set `self.TriggerCooldownHandle` _returnvalue))

(event `ControlTheControl`
  (params (bIsControlled :type Boolean))
  (`MaterialInstanceDynamic.SetVectorParameterValue` (`self.M_Control_Instance`) "Color" (`KismetMathLibrary.SelectColor` (`self.ControlledColor`) (`self.DefaultControlColor`) bIsControlled)))

(event `ChangeControlColor`
  (params (Color :type "LinearColor Structure"))
  (`MaterialInstanceDynamic.SetVectorParameterValue` (`self.M_Control_Instance`) "Color" Color))

(event `self.ReceiveTick`
  (params (DeltaSeconds :type "Float (single-precision)"))
  (switch `/Game/Blueprints/Other/Enum_ObstacleType` (`self.ObstacleType`)
    (:`NewEnumerator0`
      (`self.HandleActivatedDisabledWidget`))))

(event `self.FinishCooldown`)

(event `TriggerCooldownFinished`
  (`KismetSystemLibrary.K2_ClearAndInvalidateTimerHandle` (`self.TriggerCooldownHandle`)))

(fn `HandleActivatedDisabledWidget`
  (bind _deactivationcooldownhandle (`self.DeactivationCooldownHandle`))
  (bind _triggercooldownhandle (`self.TriggerCooldownHandle`))
  (bind _asw_trap_data (cast `/Game/UI/Widgets/W_TrapData` (`WidgetComponent.GetUserWidgetObject` (`self.Widget`)) :!pure true))
  (`|ExecutionSequence`
    (:`then_0`
      (if (`KismetSystemLibrary.K2_IsTimerActiveHandle` _deactivationcooldownhandle)
        (set `/Game/UI/Widgets/W_TrapData.IsDeactivationProgressVisible` true _asw_trap_data)
        (set `/Game/UI/Widgets/W_TrapData.DeactivationPercent` (/ (`KismetSystemLibrary.K2_GetTimerElapsedTimeHandle` _deactivationcooldownhandle) (`self.DeactivationTime`)) _asw_trap_data)
        (else
          (set `/Game/UI/Widgets/W_TrapData.IsDeactivationProgressVisible` false _asw_trap_data))))
    (:`then_1`
      (if (`KismetSystemLibrary.K2_IsTimerActiveHandle` _triggercooldownhandle)
        (set `/Game/UI/Widgets/W_TrapData.IsTriggerCooldownProgressVisible` true _asw_trap_data)
        (set `/Game/UI/Widgets/W_TrapData.TriggerCooldownPercent` (/ (`KismetSystemLibrary.K2_GetTimerElapsedTimeHandle` _triggercooldownhandle) (`self.TriggerCooldown`)) _asw_trap_data)
        (else
          (set `/Game/UI/Widgets/W_TrapData.IsTriggerCooldownProgressVisible` false _asw_trap_data))))))

(fn `HandleControlledWidget`)

(fn `UserConstructionScript`
  (`SceneComponent.SetWorldScale3D` (`self.ControlObject`) (1.0 1.0 1.0)))