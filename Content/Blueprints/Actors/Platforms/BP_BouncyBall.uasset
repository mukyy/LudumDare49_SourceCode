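; BP_BouncyBall is a bouncy obstacle actor in the platforms folder, though its bounce logic is currently disconnected.
; The construction script gives the Obstacle component a dynamic M_FlatColor material, applying its texture and a palette color chosen by ColorIndex.
; The Obstacle hit event does nothing; the unwired branch would send BounceMessage with BounceVelocity to actors implementing BPI_AIPawns.
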(event `self.Obstacle.OnComponentHit`
  (params (HitComponent :type "PrimitiveComponent Object Reference") (OtherActor :type "Actor Object Reference") (OtherComp :type "PrimitiveComponent Object Reference") (NormalImpulse :type "Vector Structure") (Hit :type "HitResult Structure (by ref)")))

(fn `UserConstructionScript`
  (`parent.UserConstructionScript`)
  (bind _returnvalue (`PrimitiveComponent.CreateDynamicMaterialInstance` (`self.Obstacle`) 0 "/Game/Materials/M_FlatColor.M_FlatColor" "None"))
  (bind _output_get (set `self.ObstacleInstance` _returnvalue))
  (`MaterialInstanceDynamic.SetTextureParameterValue` _output_get "DiffuseTexture" (`self.ObstacleTexture`))
  (`MaterialInstanceDynamic.SetVectorParameterValue` _output_get "Color" (`/Game/Blueprints/Other/BPL_Getters.GetColorPalette` (`self.ColorIndex`))))