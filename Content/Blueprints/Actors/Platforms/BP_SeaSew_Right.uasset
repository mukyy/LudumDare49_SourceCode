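; BP_SeaSew_Right is a controllable seesaw platform obstacle that tilts with mouse movement while active.
; Activate calls ControlTheControl, turns off physics on the Obstacle and opens a Tick gate that adds local roll from vertical mouse delta.
; Deactivate closes the gate and hands the Obstacle back to physics simulation.
; The construction script resets both sides to unit world scale; an alternative torque-based rotation is left unconnected.
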(event `self.ReceiveTick`
  (params (DeltaSeconds :type "Float (single-precision)"))
  (`parent.ReceiveTick` DeltaSeconds)
  (`|ExecutionSequence`
    (:`then_1`
      (`/Engine/EditorBlueprintResources/StandardMacros.Gate` true :!label _label
        (:`Exit`
          (`SceneComponent.K2_AddLocalRotation` (`self.Obstacle`) (`KismetMathLibrary.MakeRotator` (* 5.0 (`.DeltaY` (`PlayerController.GetInputMouseDelta` (`GameplayStatics.GetPlayerController` 0))))) false false))))))

(event `self.Activate`
  (set `self.IsActive` true)
  (`self.ControlTheControl` true)
  (`PrimitiveComponent.SetSimulatePhysics` (`self.Obstacle`) false)
  (goto _label :!via `Open`))

(event `self.Deactivate`
  (set `self.IsActive` false)
  (`self.ControlTheControl` false)
  (`PrimitiveComponent.SetSimulatePhysics` (`self.Obstacle`) true)
  (goto _label :!via `Close`))

(event `self.ControlObject.OnReleased`
  (params (TouchedComponent :type "PrimitiveComponent Object Reference") (ButtonReleased :type "Key Structure")))

(fn `UserConstructionScript`
  (`parent.UserConstructionScript`)
  (`SceneComponent.SetWorldScale3D` (`self.LeftSide`) (1.0 1.0 1.0))
  (`SceneComponent.SetWorldScale3D` (`self.RightSide`) (1.0 1.0 1.0)))