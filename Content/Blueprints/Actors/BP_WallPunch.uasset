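; Wall punch trap that repeatedly thrusts PunchPart out to bounce AI pawns it hits.
; From BeginPlay it loops: warn, wait TriggerRate, play the PunchAnim timeline, restart, polling while inactive.
; Each timeline update moves the part along local Y and box-traces around it, sending BounceMessage through BPI_AIPawns with a forward impulse.
; Deactivate stops the loop for a timed cooldown, then warns before re-enabling, extending the parent's cooldown events.
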(event `self.ReceiveBeginPlay`
  (`parent.ReceiveBeginPlay`)
  (`self.Activate`))

(event `self.Activate`
  (bind _punchpart (`self.PunchPart`))
  (bind _returnvalue (`SceneComponent.K2_GetComponentLocation` _punchpart))
  (if (`self.IsActive`) :!label _label
    (`self.WarnPlayer`)
    (`KismetSystemLibrary.Delay` (`self.TriggerRate`))
    (if (`self.IsActive`)
      (bind (_direction _punchalpha) (`Timeline|PunchAnim` :!via `PlayFromStart`)
        (:`Update`
          (`SceneComponent.K2_SetRelativeLocation` _punchpart (`KismetMathLibrary.MakeVector` 0.0 (`KismetMathLibrary.Lerp` 0.0 (`self.WallLength`) _punchalpha) -500.0) false false)
          (bind _outhit (`KismetSystemLibrary.BoxTraceSingle` :`Start` _returnvalue :`End` _returnvalue :`HalfSize` (* (`.BoxExtent` (`KismetSystemLibrary.GetComponentBounds` (`self.PunchPart`))) 1.2) :`TraceChannel` "TraceTypeQuery1" :`DrawDebugType` "ForOneFrame"))
          (bind (_bblockinghit _binitialoverlap _time _distance _location _impactpoint _normal _impactnormal _physmat _hitactor) (`GameplayStatics.BreakHitResult` _outhit))
          (if (`KismetSystemLibrary.DoesImplementInterface` _hitactor "/Game/Blueprints/Actors/BPI_AIPawns.BPI_AIPawns_C")
            (`KismetSystemLibrary.PrintString` "xcvcxv")
            (message `/Game/Blueprints/Actors/BPI_AIPawns.Bounce` _hitactor (* (`SceneComponent.GetForwardVector` (`self.PunchPart`)) (`self.PunchPower`)))))
        (:`Finished`
          (`self.Activate`)))
      (else
        (goto _label)))
    (else
      (`KismetSystemLibrary.Delay` 0.2)
      (goto _label))))

(event `self.Deactivate`
  (set `self.IsActive` false)
  (`self.EnterCooldown`))

(event `self.EnterCooldown`
  (`parent.EnterCooldown`)
  (bind _returnvalue (`KismetSystemLibrary.K2_SetTimerDelegate` (delegate `self.FinishCooldown`) (`self.DeactivationTime`)))
  (set `self.DeactivationCooldownHandle` _returnvalue))

(event `self.FinishCooldown`
  (`parent.FinishCooldown`)
  (`self.WarnAboutCooldown`)
  (`KismetSystemLibrary.Delay` 1.5)
  (set `self.IsActive` true))

(event `self.PunchPart.OnComponentHit`
  (params (HitComponent :type "PrimitiveComponent Object Reference") (OtherActor :type "Actor Object Reference") (OtherComp :type "PrimitiveComponent Object Reference") (NormalImpulse :type "Vector Structure") (Hit :type "HitResult Structure (by ref)"))
  (`KismetSystemLibrary.PrintString` "asdsad"))

(fn `UserConstructionScript`
  (`parent.UserConstructionScript`)
  (`SceneComponent.SetWorldScale3D` (`self.Arrow`) (1.0 1.0 1.0)))