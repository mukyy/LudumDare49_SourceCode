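; BP_CloneDevice is an actor that spawns TopDownCharacter AI pawns while any actor overlaps its Box component.
; Each Tick it polls the box's overlapping actors and spawns one pawn at a random point within the box extent around the actor's location.
; A running counter, never decremented here, stops spawning once it exceeds MaxSpawnCount.
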(event `self.ReceiveTick`
  (params (DeltaSeconds :type "Float (single-precision)"))
  (if (> (`self.CurrentSpawned`) (`self.MaxSpawnCount`))
    _
    (elif (> (`KismetArrayLibrary.Array_Length` (`PrimitiveComponent.GetOverlappingActors` (`self.Box`) null)) 0)
      (`AIBlueprintHelperLibrary.SpawnAIFromClass` "/Game/Blueprints/Actors/TopDownCharacter.TopDownCharacter_C" null (`KismetMathLibrary.RandomPointInBoundingBox` (`self.K2_GetActorLocation`) (`BoxComponent.GetScaledBoxExtent` (`self.Box`))) (struct) false null)
      (`/Engine/EditorBlueprintResources/StandardMacros.IncrementInt` (`self.CurrentSpawned`)))))

(fn `UserConstructionScript`)