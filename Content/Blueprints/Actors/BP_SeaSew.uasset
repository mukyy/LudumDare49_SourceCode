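; BP_SeaSew is a seesaw-style obstacle actor that the player tilts with horizontal mouse movement while it is activated.
; Trigger opens a gate on Tick, and releasing ControlObject closes it.
; While the gate is open, Tick applies pitch-axis torque to Obstacle proportional to mouse X delta, as an acceleration change, and prints that delta.
; The construction script resets both side components to unit world scale.
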(event `self.ReceiveTick`
  (params (DeltaSeconds :type "Float (single-precision)"))
  (bind _deltax (`PlayerController.GetInputMouseDelta` (`GameplayStatics.GetPlayerController` 0)))
  (`parent.ReceiveTick` DeltaSeconds)
  (`/Engine/EditorBlueprintResources/StandardMacros.Gate` true :!label _label
    (:`Exit`
      (`KismetSystemLibrary.PrintString` (`KismetStringLibrary.Conv_DoubleToString` _deltax))
      (`PrimitiveComponent.AddTorqueInDegrees` (`self.Obstacle`) (`KismetMathLibrary.MakeVector` 0.0 (* 2000.0 _deltax)) "None" true))))

(event `self.Activate`
  (goto _label :!via `Open`))

(event `self.Deactivate`
  (goto _label :!via `Close`))

(event `self.Trigger`
  (`self.Activate`))

(event `self.ControlObject.OnReleased`
  (params (TouchedComponent :type "PrimitiveComponent Object Reference") (ButtonReleased :type "Key Structure"))
  (`self.Deactivate`))

(fn `UserConstructionScript`
  (`parent.UserConstructionScript`)
  (`SceneComponent.SetWorldScale3D` (`self.LeftSide`) (1.0 1.0 1.0))
  (`SceneComponent.SetWorldScale3D` (`self.RightSide`) (1.0 1.0 1.0)))