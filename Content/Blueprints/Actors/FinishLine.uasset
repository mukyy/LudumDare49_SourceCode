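; Finish line actor that starts an end-of-level countdown when a pawn implementing BPI_AIPawns first enters its Box.
; A DoOnce-gated overlap creates the W_HUD widget, flags its countdown as started and sets a short one-shot timer.
; Tick copies the timer's remaining time into the HUD without checking that the widget exists yet.
; When the timer expires, LevelFinished adds the W_LevelFinish widget to the viewport.
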(event `self.ReceiveTick`
  (params (DeltaSeconds :type "Float (single-precision)"))
  (set `/Game/UI/Widgets/W_HUD.RemainingTime` (`KismetSystemLibrary.K2_GetTimerRemainingTimeHandle` (`self.CountdownHandle`)) (`self.W_HUD`)))

(event `self.Box.OnComponentBeginOverlap`
  (params (OverlappedComponent :type "PrimitiveComponent Object Reference") (OtherActor :type "Actor Object Reference") (OtherComp :type "PrimitiveComponent Object Reference") (OtherBodyIndex :type Integer) (bFromSweep :type Boolean) (SweepResult :type "HitResult Structure (by ref)"))
  (if (`KismetSystemLibrary.DoesImplementInterface` OtherActor "/Game/Blueprints/Actors/BPI_AIPawns.BPI_AIPawns_C")
    (`/Engine/EditorBlueprintResources/StandardMacros.DoOnce` false
      (:`Completed`
        (bind _returnvalue (`|CreateWidget` "/Game/UI/Widgets/W_HUD.W_HUD_C" (`GameplayStatics.GetPlayerController` 0)))
        (set `self.W_HUD` _returnvalue)
        (`UserWidget.AddToViewport` _returnvalue 0)
        (set `/Game/UI/Widgets/W_HUD.IsCountDownStarted` true _returnvalue)
        (bind _returnvalue_2 (`KismetSystemLibrary.K2_SetTimerDelegate` (delegate `LevelFinished`) 5.0))
        (set `self.CountdownHandle` _returnvalue_2)))))

(event `LevelFinished`
  (bind _returnvalue (`|CreateWidget` "/Game/UI/Widgets/W_LevelFinish.W_LevelFinish_C"))
  (`UserWidget.AddToViewport` _returnvalue 3))

(fn `UserConstructionScript`)