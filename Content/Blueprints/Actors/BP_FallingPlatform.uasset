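; BP_FallingPlatform is a cyclic moving hazard that, despite its name, slides MovingPart along local X at a fixed Z offset.
; From BeginPlay, Activate warns the player, waits TriggerRate, plays the PunchAnim timeline to drive the motion, then repeats.
; While inactive, Activate polls on a short delay.
; Deactivate starts a timed cooldown, which ends with a warning before reactivation.
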(event `self.ReceiveBeginPlay`
  (`parent.ReceiveBeginPlay`)
  (`self.Activate`))

(event `self.Activate`
  (if (`self.IsActive`) :!label _label
    (`self.WarnPlayer`)
    (`KismetSystemLibrary.Delay` (`self.TriggerRate`))
    (if (`self.IsActive`)
      (bind (_direction _punchalpha) (`Timeline|PunchAnim` :!via `PlayFromStart`)
        (:`Update`
          (`SceneComponent.K2_SetRelativeLocation` (`self.MovingPart`) (`KismetMathLibrary.MakeVector` (`KismetMathLibrary.Lerp` 0.0 500.0 _punchalpha) 0.0 -500.0) false false))
        (:`Finished`
          (`self.Activate`)))
      (else
        (goto _label)))
    (else
      (`KismetSystemLibrary.Delay` 0.2)
      (goto _label))))

(event `self.Deactivate`
  (set `self.IsActive` false)
  (`self.EnterCooldown`))

(event `self.EnterCooldown`
  (`parent.EnterCooldown`)
  (`KismetSystemLibrary.K2_SetTimerDelegate` (delegate `self.FinishCooldown`) (`self.DeactivationTime`)))

(event `self.FinishCooldown`
  (`self.WarnAboutCooldown`)
  (`KismetSystemLibrary.Delay` 1.5)
  (set `self.IsActive` true))

(fn `UserConstructionScript`
  (`parent.UserConstructionScript`)
  (`SceneComponent.SetWorldScale3D` (`self.Arrow`) (1.0 1.0 1.0)))